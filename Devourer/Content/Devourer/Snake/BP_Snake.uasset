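; Snake Blueprint for the Devourer game that connects the snake's state to the score HUD and game-over screen.
; BeginPlay adds a WBP_GameBar widget to the viewport, and Tick pushes Points and Speed into it.
; When IsLose is set, Tick instead calls Pause, adds a WBP_GameOver widget and shows the mouse cursor, with no one-shot guard in the graph.
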(event `self.ReceiveBeginPlay`
  (`self.CreateScoreWidget`))

(event `self.ReceiveTick`
  (params (DeltaSeconds :type "Float (single-precision)"))
  (if (`self.bIsLose`)
    (`self.Pause`)
    (`self.CreateGameOverWidget`)
    (else
      (`/Game/Devourer/UI/WBP_GameBar.SetScore` (`self.ScoreWudget`) (`self.Points`) (`KismetMathLibrary.Conv_IntToDouble` (`self.Speed`))))))

(fn `CreateGameOverWidget`
  (bind _returnvalue (`GameplayStatics.GetPlayerController` 0))
  (bind _returnvalue_2 (`|CreateWidget` "/Game/Devourer/UI/WBP_GameOver.WBP_GameOver_C" _returnvalue))
  (`UserWidget.AddToViewport` _returnvalue_2 0)
  (set `PlayerController.bShowMouseCursor` true _returnvalue))

(fn `CreateScoreWidget`
  (bind _returnvalue (`|CreateWidget` "/Game/Devourer/UI/WBP_GameBar.WBP_GameBar_C" (`GameplayStatics.GetPlayerController` 0)))
  (bind _output_get (set `self.ScoreWudget` _returnvalue))
  (`UserWidget.AddToViewport` _output_get 0))

(fn `UserConstructionScript`)